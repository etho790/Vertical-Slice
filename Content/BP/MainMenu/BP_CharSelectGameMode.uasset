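; Game mode for the two-player character select screen, creating both local players and gathering tagged checkpoint actors for each on BeginPlay.
; SpawnPlayerCS destroys the controller's current pawn, spawns that player's character-select pawn at a random checkpoint and possesses it.
; DespawnPlayerCS does the reverse, swapping in an InitPawn.
; Both events branch on controller ID and blend the view to that player's game camera.
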(event Custom|DespawnPlayerCS
  (params (PlayerController :type Player%20Controller%20Object%20Reference))
  (bind _returnvalue (Game|GetPlayerController 1))
  (bind _returnvalue_2 (Game|GetPlayerController 0))
  (bind _returnvalue_3 (Class|GameplayStatics|GetPlayerControllerID PlayerController))
  (bind _returnvalue_4 (Pawn|GetControlledPawn PlayerController))
  (bind _checkpointp1 (Variables|Default|GetCheckPointP1))
  (bind _checkpointp2 (Variables|Default|GetCheckPointP2))
  (Utilities|IsValid _returnvalue_4
    (:Is%20Valid
      (Actor|DestroyActor _returnvalue_4)
      (if (== _returnvalue_3 0)
        (bind _returnvalue_5 (Game|SpawnActorfromClass "/Game/BP/InitPawn.InitPawn_C" (Transformation|GetActorTransform (Utilities|Array|Get(acopy) _checkpointp1 (Math|Random|RandomIntegerinRange 0 (- (Utilities|Array|Length _checkpointp1) 1)))) "Undefined" 0 0))
        (Pawn|Possess _returnvalue_2 _returnvalue_5)
        (Game|Player|SetViewTargetwithBlend _returnvalue_2 (Variables|Default|GetGameCamera) 0.0 "VTBlend_Linear" 0.0 false)
        (elif (== _returnvalue_3 1)
          (bind _returnvalue_6 (Game|SpawnActorfromClass "/Game/BP/InitPawn.InitPawn_C" (Transformation|GetActorTransform (Utilities|Array|Get(acopy) _checkpointp2 (Math|Random|RandomIntegerinRange 0 (- (Utilities|Array|Length _checkpointp2) 1)))) "Undefined" 0 0))
          (Pawn|Possess _returnvalue _returnvalue_6)
          (Game|Player|SetViewTargetwithBlend _returnvalue (Variables|Default|GetGameCamera2) 0.0 "VTBlend_Linear" 0.0 false))))))

(event Custom|SpawnPlayerCS
  (params (PlayerController :type Player%20Controller%20Object%20Reference))
  (bind _returnvalue (Pawn|GetControlledPawn PlayerController))
  (bind _returnvalue_2 (Class|GameplayStatics|GetPlayerControllerID PlayerController))
  (bind _asbpplayer_controller_base (Utilities|Casting|CastToBPPlayerControllerBase PlayerController))
  (bind _checkpointp1 (Variables|Default|GetCheckPointP1))
  (bind _checkpointp2 (Variables|Default|GetCheckPointP2))
  (Utilities|IsValid _returnvalue
    (:Is%20Valid
      (Actor|DestroyActor _returnvalue)
      (if (== _returnvalue_2 0)
        (bind _returnvalue_3 (Game|SpawnActorfromClass "/Game/BP/MainMenu/CharSelect1.CharSelect1_C" (Transformation|GetActorTransform (Utilities|Array|Get(acopy) _checkpointp1 (Math|Random|RandomIntegerinRange 0 (- (Utilities|Array|Length _checkpointp1) 1)))) "Undefined" 0 0))
        (Pawn|Possess (Game|GetPlayerController 0) _returnvalue_3)
        (Game|Player|SetViewTargetwithBlend _asbpplayer_controller_base (Variables|Default|GetGameCamera) 0.0 "VTBlend_Linear" 0.0 false)
        (elif (== _returnvalue_2 1)
          (bind _returnvalue_4 (Game|SpawnActorfromClass "/Game/BP/MainMenu/CharSelect2.CharSelect2_C" (Transformation|GetActorTransform (Utilities|Array|Get(acopy) _checkpointp2 (Math|Random|RandomIntegerinRange 0 (- (Utilities|Array|Length _checkpointp2) 1)))) "Undefined" 0 0))
          (Pawn|Possess (Game|GetPlayerController 1) _returnvalue_4)
          (Game|Player|SetViewTargetwithBlend _asbpplayer_controller_base (Variables|Default|GetGameCamera2) 0.0 "VTBlend_Linear" 0.0 false))))))

(event EventBeginPlay
  (Utilities|FlowControl|Sequence
    (:then_0
      (bind _outactors (Actor|GetAllActorswithTag "CheckPoint_P1"))
      (Variables|Default|SetCheckPointP1 _outactors)
      (bind _outactors_2 (Actor|GetAllActorswithTag "CheckPoint_P2"))
      (Variables|Default|SetCheckPointP2 _outactors_2)
      (bind _returnvalue (Class|GameplayStatics|CreatePlayer -1))
      (Variables|Default|SetPlayer1 _returnvalue)
      (bind _returnvalue_2 (Class|GameplayStatics|CreatePlayer 0))
      (Variables|Default|SetPlayer2 _returnvalue_2))
    (:then_1
      (Input|SetInputModeGameOnly (Game|GetPlayerController 0)))))

(event EventTick
  (params (DeltaSeconds :type Float%20%28single-precision%29)))

(fn ConstructionScript)