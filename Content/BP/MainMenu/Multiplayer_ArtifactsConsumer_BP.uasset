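; Multiplayer artifact consumer actor that converts a player's carried artifacts into battle mode points.
; When a MainCharacter_BP that has picked up a powerup overlaps its sphere, it spawns a stretched shock effect below itself, plays an explosion sound and calls PowerUpPoints.
; That function awards points and clears the three regular pickup flags together, checking the higher-scoring most powerful artifact only when none of those are held.
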(event OnComponentBeginOverlap(Sphere)
  (params (OverlappedComponent :type Primitive%20Component%20Object%20Reference) (OtherActor :type Actor%20Object%20Reference) (OtherComp :type Primitive%20Component%20Object%20Reference) (OtherBodyIndex :type Integer) (bFromSweep :type Boolean) (SweepResult :type Hit%20Result%20Structure%20%28by%20ref%29))
  (bind _self self)
  (bind _returnvalue (Transformation|GetActorLocation _self))
  (bind _asmain_character_bp (Utilities|Casting|CastToMainCharacter_BP OtherActor))
  (if (Variables|/Script/MyTemplate.CharacterBase|GetHasPickedUpPowerup _asmain_character_bp)
    (Game|SpawnActorfromClass "/Game/BP/PrazmaShockArtifactsConsumer.PrazmaShockArtifactsConsumer_C" (Math|Transform|MakeTransform (- _returnvalue "0, 0,200.000000") "0, 0, 0" "2.500000,2.500000,15.000000") "Undefined" 0 0)
    (Audio|PlaySoundatLocation "/Game/Sound/MSoundFiles/BombExplo.BombExplo" _returnvalue "0, 0, 0" 1.0 1.0 0.0 0 0 0)
    ;[1 1 1] CONVERTS ALL THE ARTIFACTS TO POINTS
    (CallFunction|PowerUpPoints _asmain_character_bp _asmain_character_bp _asmain_character_bp _asmain_character_bp _asmain_character_bp _asmain_character_bp _asmain_character_bp _asmain_character_bp)))

(event EventBeginPlay)

(event Collision|EventActorBeginOverlap
  (params (OtherActor :type Actor%20Object%20Reference)))

(event EventTick
  (params (DeltaSeconds :type Float%20%28single-precision%29)))

(fn ConstructionScript)

(fn PowerUpPoints
  (params (self2 :type Character%20Base%20Object%20Reference) (self3 :type Character%20Base%20Object%20Reference) (self4 :type Character%20Base%20Object%20Reference) (self5 :type Character%20Base%20Object%20Reference) (self6 :type Main%20Character%20BP%20Object%20Reference) (self7 :type Main%20Character%20BP%20Object%20Reference) (self8 :type Main%20Character%20BP%20Object%20Reference) (self9 :type Main%20Character%20BP%20Object%20Reference))
  (if (Math|Boolean|ORBoolean (Variables|/Script/MyTemplate.CharacterBase|GetHomingMissilePicked self3) (Variables|/Script/MyTemplate.CharacterBase|GetFlashBombPicked self4) (Variables|/Script/MyTemplate.CharacterBase|GetThirdPickup self5))
    (Variables|/Game/BP/Characters/MainCharacter_BP.MainCharacter_BP_C|SetBattleMode_TotalPoints self6 (+ (Variables|/Game/BP/Characters/MainCharacter_BP.MainCharacter_BP_C|GetBattleMode_TotalPoints self7) 20))
    (Variables|/Script/MyTemplate.CharacterBase|SetHomingMissilePicked self2 false)
    (Variables|/Script/MyTemplate.CharacterBase|SetFlashBombPicked self2 false)
    (Variables|/Script/MyTemplate.CharacterBase|SetThirdPickup self2 false)
    (elif (Variables|/Game/BP/Characters/MainCharacter_BP.MainCharacter_BP_C|GetBattleMode_MostPowerfulArtifact self8)
      (Variables|/Game/BP/Characters/MainCharacter_BP.MainCharacter_BP_C|SetBattleMode_TotalPoints self9 (+ (Variables|/Game/BP/Characters/MainCharacter_BP.MainCharacter_BP_C|GetBattleMode_TotalPoints self7) 60))
      (Variables|/Game/BP/Characters/MainCharacter_BP.MainCharacter_BP_C|SetBattleMode_MostPowerfulArtifact self9 false))))