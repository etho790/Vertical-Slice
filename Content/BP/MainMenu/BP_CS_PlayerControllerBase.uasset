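; Player controller for the character select screen, letting two local players join, change look and start the match.
; Gamepad Special Left or keys 1/2 spawn each player's character through BP_CharSelectGameMode, gated by controller ID.
; The bottom face button calls ChangeLook once that player is ready, and Special Right calls MatchStart.
; BeginPlay creates the HUD and grappler widgets after a short delay, without adding them to the viewport.
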(event EventBeginPlay
  ;[1 1 1] This is responsible for spawning the characters based on the controller select button, which calls the bp_character selectgamemode
  (Utilities|FlowControl|Delay 0.1)
  (bind _returnvalue (UserInterface|CreateWidget "/Game/BP/BP_MyHud.BP_MyHud_C" self))
  (Variables|Default|SetHUD _returnvalue)
  (bind _returnvalue_2 (UserInterface|CreateWidget "/Game/UI/ICONS/Grappler/Widget_Grappler.Widget_Grappler_C" self))
  (Variables|Default|SetGrappleHud _returnvalue_2))

(event Input|GamepadEvents|GamepadFaceButtonBottom
  (params (Key :type Key%20Structure :default "None"))
  ;[1 1 1] This is responsible for spawning the characters based on the controller select button, which calls the bp_character selectgamemode
  (:Pressed
    (if (Variables|/Game/BP/MainMenu/BP_CharSelectGameMode.BP_CharSelectGameMode_C|GetP1Ready (stale Input|GamepadEvents|GamepadSpecialLeft _asbp_char_select_game_mode))
      (if (== (Class|GameplayStatics|GetPlayerControllerID self) 0)
        (Default|ChangeLook (Variables|/Game/BP/MainMenu/BP_CharSelectGameMode.BP_CharSelectGameMode_C|GetCharSelect1 (stale Input|GamepadEvents|GamepadSpecialLeft _asbp_char_select_game_mode)))))))

(event Input|GamepadEvents|GamepadFaceButtonBottom
  (params (Key :type Key%20Structure :default "None"))
  ;[1 1 1] This is responsible for spawning the characters based on the controller select button, which calls the bp_character selectgamemode
  (:Pressed
    (if (Variables|/Game/BP/MainMenu/BP_CharSelectGameMode.BP_CharSelectGameMode_C|GetP2Ready (stale Input|GamepadEvents|GamepadSpecialLeft _asbp_char_select_game_mode))
      (if (== (Class|GameplayStatics|GetPlayerControllerID self) 1)
        (Default|ChangeLook (Variables|/Game/BP/MainMenu/BP_CharSelectGameMode.BP_CharSelectGameMode_C|GetcharSelect2 (stale Input|GamepadEvents|GamepadSpecialLeft _asbp_char_select_game_mode)))))))

(event Input|GamepadEvents|GamepadSpecialRight
  (params (Key :type Key%20Structure :default "None"))
  ;[1 1 1] This is responsible for spawning the characters based on the controller select button, which calls the bp_character selectgamemode
  ;;[1 1 1] Starts the match, counting down the timer
  (:Pressed
    (bind _asbp_char_select_game_mode (Utilities|Casting|CastToBP_CharSelectGameMode (Game|GetGameMode)))
    (Default|MatchStart _asbp_char_select_game_mode)))

(event Input|GamepadEvents|GamepadSpecialLeft
  (params (Key :type Key%20Structure :default "None"))
  ;[1 1 1] This is responsible for spawning the characters based on the controller select button, which calls the bp_character selectgamemode
  (:Pressed
    (bind _asbp_char_select_game_mode (Utilities|Casting|CastToBP_CharSelectGameMode (Game|GetGameMode)))
    (if (== (Class|GameplayStatics|GetPlayerControllerID self) 1)
      (Default|SpawnPlayerCS2 _asbp_char_select_game_mode (Game|GetPlayerController 1)))))

(event Input|GamepadEvents|GamepadSpecialLeft
  (params (Key :type Key%20Structure :default "None"))
  ;[1 1 1] This is responsible for spawning the characters based on the controller select button, which calls the bp_character selectgamemode
  (:Pressed
    (bind _asbp_char_select_game_mode (Utilities|Casting|CastToBP_CharSelectGameMode (Game|GetGameMode)))
    (if (== (Class|GameplayStatics|GetPlayerControllerID self) 0)
      (Default|SpawnPlayerCS1 _asbp_char_select_game_mode (Game|GetPlayerController 0)))))

(event Input|KeyboardEvents|1
  (params (Key :type Key%20Structure :default "None"))
  ;[1 1 1] This is responsible for spawning the characters based on the controller select button, which calls the bp_character selectgamemode
  (:Pressed
    (bind _asbp_char_select_game_mode (Utilities|Casting|CastToBP_CharSelectGameMode (Game|GetGameMode)))
    (if (== (Class|GameplayStatics|GetPlayerControllerID self) 0)
      (Default|SpawnPlayerCS1 _asbp_char_select_game_mode (Game|GetPlayerController 0)))))

(event Input|KeyboardEvents|2
  (params (Key :type Key%20Structure :default "None"))
  ;[1 1 1] This is responsible for spawning the characters based on the controller select button, which calls the bp_character selectgamemode
  (:Pressed
    (bind _asbp_char_select_game_mode (Utilities|Casting|CastToBP_CharSelectGameMode (Game|GetGameMode)))
    (if (== (Class|GameplayStatics|GetPlayerControllerID self) 1)
      (Default|SpawnPlayerCS2 _asbp_char_select_game_mode (Game|GetPlayerController 1)))))

(fn ConstructionScript)