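; Trigger box actor that marks where the player characters are allowed to climb.
; When an actor tagged P1 or P2 enters ClimbTrigger, it is cast to BP_MyCharacterBase and its MTriggerCanClimb flag is set true.
; Leaving the trigger sets the flag back to false.
; The climb itself is not handled here, and the debug prints are unconnected.
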(event OnComponentBeginOverlap(ClimbTrigger)
  (params (OverlappedComponent :type Primitive%20Component%20Object%20Reference) (OtherActor :type Actor%20Object%20Reference) (OtherComp :type Primitive%20Component%20Object%20Reference) (OtherBodyIndex :type Integer) (bFromSweep :type Boolean) (SweepResult :type Hit%20Result%20Structure%20%28by%20ref%29))
  (if (Actor|ActorHasTag OtherActor "P1")
    (bind _asbp_my_character_base (Utilities|Casting|CastToBP_MyCharacterBase OtherActor))
    (Variables|/Game/BP/Characters/BP_MyCharacterBase.BP_MyCharacterBase_C|SetM%20TriggerCanClimb _asbp_my_character_base true)
    (elif (Actor|ActorHasTag OtherActor "P2")
      (bind _asbp_my_character_base_2 (Utilities|Casting|CastToBP_MyCharacterBase OtherActor))
      (Variables|/Game/BP/Characters/BP_MyCharacterBase.BP_MyCharacterBase_C|SetM%20TriggerCanClimb _asbp_my_character_base_2 true))))

(event OnComponentEndOverlap(ClimbTrigger)
  (params (OverlappedComponent :type Primitive%20Component%20Object%20Reference) (OtherActor :type Actor%20Object%20Reference) (OtherComp :type Primitive%20Component%20Object%20Reference) (OtherBodyIndex :type Integer))
  (if (Actor|ActorHasTag OtherActor "P1")
    (bind _asbp_my_character_base (Utilities|Casting|CastToBP_MyCharacterBase OtherActor))
    (Variables|/Game/BP/Characters/BP_MyCharacterBase.BP_MyCharacterBase_C|SetM%20TriggerCanClimb _asbp_my_character_base false)
    (elif (Actor|ActorHasTag OtherActor "P2")
      (bind _asbp_my_character_base_2 (Utilities|Casting|CastToBP_MyCharacterBase OtherActor))
      (Variables|/Game/BP/Characters/BP_MyCharacterBase.BP_MyCharacterBase_C|SetM%20TriggerCanClimb _asbp_my_character_base_2 false))))

(event EventBeginPlay)

(event Collision|EventActorBeginOverlap
  (params (OtherActor :type Actor%20Object%20Reference)))

(event EventTick
  (params (DeltaSeconds :type Float%20%28single-precision%29)))

(fn ConstructionScript)