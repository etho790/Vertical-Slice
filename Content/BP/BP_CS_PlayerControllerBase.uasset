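; Player controller base for character select that lets local players join and handles menu widgets.
; The 1 and 2 keys or gamepad special-right ask BP_CharSelectGameMode to spawn player one or two, matched by controller ID.
; BeginPlay creates HUD and grappler widgets without displaying them.
; M or Escape toggles the in-game menu and mouse input, and C opens a name-change widget until the match has begun.
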(event EventBeginPlay
  ;[1 1 1] Ive  only taken the button presses off for the time being
  (Utilities|FlowControl|Delay 0.1)
  (bind _returnvalue (UserInterface|CreateWidget "/Game/BP/BP_MyHud.BP_MyHud_C" self))
  (Variables|Default|SetHUD _returnvalue)
  (bind _returnvalue_2 (UserInterface|CreateWidget "/Game/UI/ICONS/Grappler/Widget_Grappler.Widget_Grappler_C" self))
  (Variables|Default|SetGrappleHud _returnvalue_2))

(event Input|ActionEvents|InputActionESCFROMUI
  (params (Key :type Key%20Structure :default "None")))

(event Input|KeyboardEvents|3
  (params (Key :type Key%20Structure :default "None"))
  ;[1 1 1] Ive  only taken the button presses off for the time being
)

(event Input|KeyboardEvents|R
  (params (Key :type Key%20Structure :default "None"))
  ;[1 1 1] Ive  only taken the button presses off for the time being
)

(event Input|KeyboardEvents|C
  (params (Key :type Key%20Structure :default "None"))
  (:Pressed
    (bind _asmultiplayer_game_instance (Utilities|Casting|CastToMultiplayerGameInstance (Game|GetGameInstance)))
    (if (not (Variables|/Game/UI/M_UI/Multiplayer/MultiplayerGameInstance.MultiplayerGameInstance_C|GetHasMatchBegun _asmultiplayer_game_instance))
      (Utilities|FlowControl|Delay 0.1)
      (Utilities|IsValid (Variables|Default|GetChangePlayerName)
        (:Is%20Valid
          (if (not (UserInterface|Viewport|IsinViewport (Variables|Default|GetChangePlayerName)))
            (UserInterface|Viewport|AddtoViewport (Variables|Default|GetChangePlayerName) 0)
            (Variables|Default|SetbShowMouseCursor true)))
        (:Is%20Not%20Valid
          (bind _returnvalue (UserInterface|CreateWidget "/Game/BP/MainMenu/WB_ChangePlayerName.WB_ChangePlayerName_C"))
          (bind _output_get (Variables|Default|SetChangePlayerName _returnvalue))
          (UserInterface|Viewport|AddtoViewport _output_get 0)
          (Variables|Default|SetbShowMouseCursor true)
          (Input|SetInputModeGameandUI (Game|GetPlayerController 0) (Variables|Default|GetInGameMenu) "LockAlways" false))))))

(event Input|GamepadEvents|GamepadSpecialRight
  (params (Key :type Key%20Structure :default "None"))
  ;[1 1 1] Ive  only taken the button presses off for the time being
  (:Pressed
    (bind _asbp_char_select_game_mode (Utilities|Casting|CastToBP_CharSelectGameMode (Game|GetGameMode)))
    (if (== (Class|GameplayStatics|GetPlayerControllerID self) 0)
      (Default|SpawnPlayerCS1 _asbp_char_select_game_mode (Game|GetPlayerController 0)))))

(event Input|GamepadEvents|GamepadSpecialRight
  (params (Key :type Key%20Structure :default "None"))
  ;[1 1 1] Ive  only taken the button presses off for the time being
  (:Pressed
    (bind _asbp_char_select_game_mode (Utilities|Casting|CastToBP_CharSelectGameMode (Game|GetGameMode)))
    (if (== (Class|GameplayStatics|GetPlayerControllerID self) 1)
      (Default|SpawnPlayerCS2 _asbp_char_select_game_mode (Game|GetPlayerController 1)))))

(event Input|KeyboardEvents|Escape
  (params (Key :type Key%20Structure :default "None"))
  (bind _returnvalue (Game|GetPlayerController 0))
  (:Pressed
    (Utilities|FlowControl|Delay 0.1)
    (Utilities|IsValid (Variables|Default|GetInGameMenu)
      (:Is%20Valid
        (if (UserInterface|Viewport|IsinViewport (Variables|Default|GetInGameMenu))
          (Widget|RemovefromParent (Variables|Default|GetInGameMenu))
          (Variables|Default|SetbShowMouseCursor false)
          (Input|SetInputModeGameOnly _returnvalue)
          (else
            (bind _returnvalue_2 (UserInterface|CreateWidget "/Game/BP/MainMenu/WB_InGameMenu.WB_InGameMenu_C" :!label _label))
            (bind _output_get (Variables|Default|SetInGameMenu _returnvalue_2))
            (UserInterface|Viewport|AddtoViewport _output_get 0)
            (Variables|Default|SetbShowMouseCursor true)
            (Input|SetInputModeGameandUI _returnvalue (Variables|Default|GetInGameMenu) "DoNotLock" true))))
      (:Is%20Not%20Valid
        (goto _label)))))

(event Input|KeyboardEvents|M
  (params (Key :type Key%20Structure :default "None"))
  (bind _returnvalue (Game|GetPlayerController 0))
  (:Pressed
    (Utilities|FlowControl|Delay 0.1)
    (Utilities|IsValid (Variables|Default|GetInGameMenu)
      (:Is%20Valid
        (if (UserInterface|Viewport|IsinViewport (Variables|Default|GetInGameMenu))
          (Widget|RemovefromParent (Variables|Default|GetInGameMenu))
          (Variables|Default|SetbShowMouseCursor false)
          (Input|SetInputModeGameOnly _returnvalue)
          (else
            (bind _returnvalue_2 (UserInterface|CreateWidget "/Game/BP/MainMenu/WB_InGameMenu.WB_InGameMenu_C" :!label _label))
            (bind _output_get (Variables|Default|SetInGameMenu _returnvalue_2))
            (UserInterface|Viewport|AddtoViewport _output_get 0)
            (Variables|Default|SetbShowMouseCursor true)
            (Input|SetInputModeGameandUI _returnvalue (Variables|Default|GetInGameMenu) "DoNotLock" true))))
      (:Is%20Not%20Valid
        (goto _label)))))

(event Input|GamepadEvents|GamepadSpecialLeft
  (params (Key :type Key%20Structure :default "None"))
  ;[1 1 1] Ive  only taken the button presses off for the time being
)

(event Input|KeyboardEvents|Escape
  (params (Key :type Key%20Structure :default "None")))

(event Input|KeyboardEvents|1
  (params (Key :type Key%20Structure :default "None"))
  ;[1 1 1] Ive  only taken the button presses off for the time being
  (:Pressed
    (bind _asbp_char_select_game_mode (Utilities|Casting|CastToBP_CharSelectGameMode (Game|GetGameMode)))
    (if (== (Class|GameplayStatics|GetPlayerControllerID self) 0)
      (Default|SpawnPlayerCS1 _asbp_char_select_game_mode (Game|GetPlayerController 0)))))

(event Input|KeyboardEvents|2
  (params (Key :type Key%20Structure :default "None"))
  ;[1 1 1] Ive  only taken the button presses off for the time being
  (:Pressed
    (bind _asbp_char_select_game_mode (Utilities|Casting|CastToBP_CharSelectGameMode (Game|GetGameMode)))
    (if (== (Class|GameplayStatics|GetPlayerControllerID self) 1)
      (Default|SpawnPlayerCS2 _asbp_char_select_game_mode (Game|GetPlayerController 1)))))

(event Input|KeyboardEvents|M
  (params (Key :type Key%20Structure :default "None")))

(fn ConstructionScript)