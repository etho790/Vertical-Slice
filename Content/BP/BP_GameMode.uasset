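; Game mode for a local two-player match that creates both players and handles their spawning and despawning.
; BeginPlay gathers tagged checkpoints per player, recreates the local players, spawns both after a short delay, shows a map-name widget and clears match-end flags.
; Spawn events replace an existing pawn with that player's character at a random checkpoint and add HUDs; DespawnPlayer swaps in an InitPawn and removes the main HUD.
; The training-level name check has empty branches.
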(event Custom|SpawnPlayer1
  (params (PlayerController :type Player%20Controller%20Object%20Reference))
  (bind _returnvalue (Pawn|GetControlledPawn PlayerController))
  (bind _asbpplayer_controller_base (Utilities|Casting|CastToBPPlayerControllerBase PlayerController))
  (bind _checkpointp1 (Variables|Default|GetCheckPointP1))
  (Utilities|IsValid _returnvalue
    (:Is%20Valid
      (Actor|DestroyActor _returnvalue)
      (if (== (Class|GameplayStatics|GetPlayerControllerID PlayerController) 0)
        (bind _returnvalue_2 (Game|SpawnActorfromClass "/Game/BP/Characters/PlayerOne.PlayerOne_C" (Transformation|GetActorTransform (Utilities|Array|Get(acopy) _checkpointp1 (Math|Random|RandomIntegerinRange 0 (- (Utilities|Array|Length _checkpointp1) 1)))) "Undefined" 0 0))
        (bind _output_get (Variables|Default|SetPLAYER1 _returnvalue_2))
        (Pawn|Possess (Game|GetPlayerController 0) _output_get)
        (UserInterface|Viewport|AddtoPlayerScreen (Variables|/Game/BP/BPPlayerControllerBase.BPPlayerControllerBase_C|GetHUD _asbpplayer_controller_base))
        (UserInterface|Viewport|AddtoPlayerScreen (Variables|/Game/BP/BPPlayerControllerBase.BPPlayerControllerBase_C|GetGrappleHud _asbpplayer_controller_base))))))

(event Custom|DespawnPlayer
  (params (PlayerController :type Player%20Controller%20Object%20Reference))
  (bind _returnvalue (Class|GameplayStatics|GetPlayerControllerID PlayerController))
  (bind _returnvalue_2 (Pawn|GetControlledPawn PlayerController))
  (bind _asbpplayer_controller_base (Utilities|Casting|CastToBPPlayerControllerBase PlayerController))
  (bind _checkpointp1 (Variables|Default|GetCheckPointP1))
  (bind _checkpointp2 (Variables|Default|GetCheckPointP2))
  (bind _hud (Variables|/Game/BP/BPPlayerControllerBase.BPPlayerControllerBase_C|GetHUD _asbpplayer_controller_base))
  (Utilities|IsValid _returnvalue_2
    (:Is%20Valid
      (Actor|DestroyActor _returnvalue_2)
      (if (== _returnvalue 0)
        (bind _returnvalue_3 (Game|SpawnActorfromClass "/Game/BP/InitPawn.InitPawn_C" (Transformation|GetActorTransform (Utilities|Array|Get(acopy) _checkpointp1 (Math|Random|RandomIntegerinRange 0 (- (Utilities|Array|Length _checkpointp1) 1)))) "Undefined" 0 0))
        (Pawn|Possess PlayerController _returnvalue_3)
        (Widget|RemovefromParent _hud)
        (elif (== _returnvalue 1)
          (bind _returnvalue_4 (Game|SpawnActorfromClass "/Game/BP/InitPawn.InitPawn_C" (Transformation|GetActorTransform (Utilities|Array|Get(acopy) _checkpointp2 (Math|Random|RandomIntegerinRange 0 (- (Utilities|Array|Length _checkpointp2) 1)))) "Undefined" 0 0))
          (Pawn|Possess PlayerController _returnvalue_4)
          (Widget|RemovefromParent _hud))))))

(event Custom|SpawnPlayer2
  (params (PlayerController :type Player%20Controller%20Object%20Reference))
  (bind _returnvalue (Pawn|GetControlledPawn PlayerController))
  (bind _asbpplayer_controller_base (Utilities|Casting|CastToBPPlayerControllerBase PlayerController))
  (bind _checkpointp2 (Variables|Default|GetCheckPointP2))
  (Utilities|IsValid _returnvalue
    (:Is%20Valid
      (Actor|DestroyActor _returnvalue)
      (if (== (Class|GameplayStatics|GetPlayerControllerID PlayerController) 1)
        (bind _returnvalue_2 (Game|SpawnActorfromClass "/Game/BP/Characters/PlayerTwo.PlayerTwo_C" (Transformation|GetActorTransform (Utilities|Array|Get(acopy) _checkpointp2 (Math|Random|RandomIntegerinRange 0 (- (Utilities|Array|Length _checkpointp2) 1)))) "Undefined" 0 0))
        (bind _output_get (Variables|Default|SetPLAYER2 _returnvalue_2))
        (Pawn|Possess (Game|GetPlayerController 1) _output_get)
        (UserInterface|Viewport|AddtoPlayerScreen (Variables|/Game/BP/BPPlayerControllerBase.BPPlayerControllerBase_C|GetHUD _asbpplayer_controller_base))
        (UserInterface|Viewport|AddtoPlayerScreen (Variables|/Game/BP/BPPlayerControllerBase.BPPlayerControllerBase_C|GetGrappleHud _asbpplayer_controller_base))))))

(event EventBeginPlay
  (Utilities|FlowControl|Sequence
    (:then_0
      (Class|GameplayStatics|RemovePlayer (Game|GetPlayerController 1) false))
    (:then_1
      (Utilities|FlowControl|Sequence
        (:then_0
          (bind _outactors (Actor|GetAllActorswithTag "CheckPoint_P1"))
          (Variables|Default|SetCheckPointP1 _outactors)
          (bind _outactors_2 (Actor|GetAllActorswithTag "CheckPoint_P2"))
          (Variables|Default|SetCheckPointP2 _outactors_2)
          (bind _returnvalue (Class|GameplayStatics|CreatePlayer -1))
          (Variables|Default|Setp1 _returnvalue)
          (bind _returnvalue_2 (Class|GameplayStatics|CreatePlayer 0 false))
          (Variables|Default|Setp2 _returnvalue_2)
          (Utilities|FlowControl|Delay 0.2)
          (CallFunction|SpawnPlayer1 (Game|GetPlayerController 0))
          ;[1 1 1] Enochs Code for training level map
          (bind _returnvalue_3 (Game|GetCurrentLevelName true))
          (if (Utilities|Enum|Equal(Enum) _returnvalue_3 "TrainingLevelMap")
            _
            (else
              _))
          (CallFunction|SpawnPlayer2 (Game|GetPlayerController 1)))))
    (:then_2
      (bind _returnvalue_4 (UserInterface|CreateWidget "/Game/BP/MapNameStart.MapNameStart_C"))
      (UserInterface|Viewport|AddtoViewport _returnvalue_4 0))
    (:then_3
      (Variables|Default|SetMatchEndP1 false)
      (Variables|Default|SetMatchEndP2 false))))

(fn ConstructionScript)