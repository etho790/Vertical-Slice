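; Flash bomb power-up pickup that either of two players can collect by touching it.
; The mesh spins every tick with an orbit particle effect attached.
; On sphere overlap, a P1 or P2 tagged player not already holding something gets its FlashBombPickUp flag set; the pickup then spawns a particle effect, plays a sound and destroys itself.
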(event OnComponentBeginOverlap(Sphere)
  (params (OverlappedComponent :type Primitive%20Component%20Object%20Reference) (OtherActor :type Actor%20Object%20Reference) (OtherComp :type Primitive%20Component%20Object%20Reference) (OtherBodyIndex :type Integer) (bFromSweep :type Boolean) (SweepResult :type Hit%20Result%20Structure%20%28by%20ref%29))
  ;[1 1 1] Destroys after Collision
  (if (Actor|ActorHasTag OtherActor "P1")
    (bind _asplayer_one (Utilities|Casting|CastToPlayerOne OtherActor))
    (if (not (Variables|/Game/BP/Characters/PlayerOne.PlayerOne_C|GetHasPickedUpSomething _asplayer_one))
      (Variables|/Game/BP/Characters/PlayerOne.PlayerOne_C|SetFlashBombPickUp _asplayer_one true)
      ;[1 1 1] DISENTEGRATION PS here
      (Effects|SpawnEmitteratLocation "/Game/Particles/Effects/PS_Pickup.PS_Pickup" (Transformation|GetWorldLocation (Variables|Default|GetSM_FlashBomb)) :!label _label)
      (Audio|PlaySound2D "/Game/Sound/MSoundFiles/PickUps.PickUps" 1.0 1.0 0.0 0 0)
      (Actor|DestroyActor))
    (elif (Actor|ActorHasTag OtherActor "P2")
      (bind _asplayer_two (Utilities|Casting|CastToPlayerTwo OtherActor))
      (if (not (Variables|/Game/BP/Characters/PlayerTwo.PlayerTwo_C|GethasPickedUpSomething _asplayer_two))
        (Variables|/Game/BP/Characters/PlayerTwo.PlayerTwo_C|SetFlashBombPickUp _asplayer_two true)
        (goto _label)))))

(event EventBeginPlay
  (bind _returnvalue (Transformation|GetActorTransform))
  ;[1 1 1] begin play
  (Variables|Default|SetStarting%20Pos (.location _returnvalue))
  (Variables|Default|SetStarting%20Rotation (Math|Rotator|GetRotationXVector (.rotation _returnvalue)))
  (Effects|SpawnEmitterAttached "/Game/PowerUps/FlashBomb/Particles/PS_Orbit.PS_Orbit" (Variables|Default|GetSM_FlashBomb) "None"))

(event EventTick
  (params (DeltaSeconds :type Float%20%28single-precision%29))
  (bind _starting_rotation (Variables|Default|GetStarting%20Rotation))
  ;[1 1 1] Just powerup Rotation and Translation
  (Transformation|AddLocalRotation (Variables|Default|GetSM_FlashBomb) (Math|Rotator|MakeRotator (+ (.x _starting_rotation) 1.5) (+ (.y _starting_rotation) 2.0) (+ (.z _starting_rotation) 0.5)) false false))

(fn ConstructionScript)