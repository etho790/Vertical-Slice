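; Flash bomb weapon actor that blinds either of the two players caught within its radius.
; BeginPlay caches both players from BP_GameMode and sets the maximum effect distance.
; Tick spawns an actor at the bomb mesh, calls FlashBomb on each player in range, clears their UsersFlashBomb flag, then destroys itself.
; A second Tick branch handles missing players with a delayed flag reset and destroy.
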(event EventBeginPlay
  ;[1 1 1] GameMode
  (bind _asbp_game_mode (Utilities|Casting|CastToBP_GameMode (Game|GetGameMode)))
  (bind _output_get (Variables|Default|SetGameMode _asbp_game_mode))
  (Variables|Default|SetPlayer2 (Variables|/Game/BP/BP_GameMode.BP_GameMode_C|GetPLAYER2 _output_get))
  (Variables|Default|SetPlayer1 (Variables|/Game/BP/BP_GameMode.BP_GameMode_C|GetPLAYER1 _output_get))
  (Variables|Default|SetMaxDistanceFromFlashBomb 1.5e+03))

(event EventTick
  (params (DeltaSeconds :type Float%20%28single-precision%29))
  (bind _player1 (Variables|Default|GetPlayer1))
  (bind _player2 (Variables|Default|GetPlayer2))
  (Utilities|FlowControl|Sequence
    (:then_0
      ;[1 1 1] Length of delay, Spawning of explosion decal on ground and destroy actor
      (Game|SpawnActorfromClass "/Game/PowerUps/FlashBomb/BP/BP_ExplosionDecal.BP_ExplosionDecal_C" (Math|Transform|MakeTransform (Transformation|GetWorldLocation (Variables|Default|GetSM_FlashBomb)) "0, 0, 0" "1,1,1") "Undefined" 0 0)
      (Utilities|FlowControl|Sequence
        (:then_0
          (if (not (>= (Math|Vector|VectorLength (- (Transformation|GetActorLocation _player1) (Transformation|GetWorldLocation (Variables|Default|GetSM_FlashBomb self)))) (Variables|Default|GetMaxDistanceFromFlashBomb)))
            (Default|FlashBomb _player1)
            (Variables|/Game/BP/Characters/PlayerOne.PlayerOne_C|SetUsersFlashBomb _player1 false)
            (Variables|Default|SetExplode false :!label _label)))
        (:then_1
          (if (not (>= (Math|Vector|VectorLength (- (Transformation|GetActorLocation _player2) (Transformation|GetWorldLocation (Variables|Default|GetSM_FlashBomb self)))) (Variables|Default|GetMaxDistanceFromFlashBomb)))
            (Default|FlashBomb _player2)
            (Variables|/Game/BP/Characters/PlayerTwo.PlayerTwo_C|SetUsersFlashBomb _player2 false)
            (goto _label)))
        (:then_2
          (Actor|DestroyActor))))
    (:then_1
      ;[1 1 1] Delete if both are null
      (if (and (== (Variables|Default|GetPlayer1) 0) (== (Variables|Default|GetPlayer2) 0))
        (Utilities|FlowControl|Delay 2.0)
        ;[1 1 1] at the end of individual players flash, the bool is set to false
        (Variables|/Game/BP/Characters/PlayerTwo.PlayerTwo_C|SetUsersFlashBomb (Variables|Default|GetPlayer2) false)
        (Variables|/Game/BP/Characters/PlayerOne.PlayerOne_C|SetUsersFlashBomb (Variables|Default|GetPlayer1) false)
        (Actor|DestroyActor)))))

(fn ConstructionScript)