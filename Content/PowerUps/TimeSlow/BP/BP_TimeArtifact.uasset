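; Time artifact power-up actor meant to grant a time slow bomb pickup, with its gameplay logic currently disconnected.
; BeginPlay caches the starting location and rotation, while Tick and box overlap do nothing.
; Unwired nodes would spin the mesh and, for a tagged P1 or P2 not already holding an item, set the pickup flag, spawn pickup particles and destroy the actor.
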(event OnComponentBeginOverlap(Box)
  (params (OverlappedComponent :type Primitive%20Component%20Object%20Reference) (OtherActor :type Actor%20Object%20Reference) (OtherComp :type Primitive%20Component%20Object%20Reference) (OtherBodyIndex :type Integer) (bFromSweep :type Boolean) (SweepResult :type Hit%20Result%20Structure%20%28by%20ref%29))
  ;[1 1 1] Destroys after Collision
)

(event EventBeginPlay
  (bind _returnvalue (Transformation|GetActorTransform))
  (Variables|Default|SetStarting%20Pos (.location _returnvalue))
  (Variables|Default|SetStarting%20Rotaion (Math|Rotator|GetRotationXVector (.rotation _returnvalue))))

(event EventTick
  (params (DeltaSeconds :type Float%20%28single-precision%29))
  ;[1 1 1] Powerup Rotation and translation
)

(fn ConstructionScript)