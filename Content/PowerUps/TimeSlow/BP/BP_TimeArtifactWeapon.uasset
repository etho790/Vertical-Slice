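; Time artifact weapon actor from the TimeSlow power-up set, currently holding only setup logic.
; On BeginPlay it caches the BP_GameMode and its PLAYER1 and PLAYER2 references, then initializes TimerExpansion.
; Tick is empty, and the nodes that spawn an explosion decal at the artifact mesh and destroy the actor are disconnected, so they never run.
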(event EventBeginPlay
  ;[1 1 1] GameMode
  (bind _asbp_game_mode (Utilities|Casting|CastToBP_GameMode (Game|GetGameMode)))
  (bind _output_get (Variables|Default|SetGameMode _asbp_game_mode))
  (Variables|Default|SetPlayer2 (Variables|/Game/BP/BP_GameMode.BP_GameMode_C|GetPLAYER2 _output_get))
  (Variables|Default|SetPlayer1 (Variables|/Game/BP/BP_GameMode.BP_GameMode_C|GetPLAYER1 _output_get))
  (Variables|Default|SetTimerExpansion 5e+01))

(event EventTick
  (params (DeltaSeconds :type Float%20%28single-precision%29))
  ;[1 1 1] Length of delay, Spawning of explosion decal on ground and destroy actor
)

(fn ConstructionScript)