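; BP_RocketJav is a spinning power-up pickup that grants the homing missile pickup to Player One or Player Two.
; It attaches a javelin particle effect on start and rotates its mesh every tick, offset by the starting rotation's forward vector and not scaled by delta time.
; Sphere overlap checks the P1/P2 tag and, if that player holds nothing, sets HomingMissilePickup, plays effects and destroys itself.
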(event OnComponentBeginOverlap(Sphere)
  (params (OverlappedComponent :type Primitive%20Component%20Object%20Reference) (OtherActor :type Actor%20Object%20Reference) (OtherComp :type Primitive%20Component%20Object%20Reference) (OtherBodyIndex :type Integer) (bFromSweep :type Boolean) (SweepResult :type Hit%20Result%20Structure%20%28by%20ref%29))
  ;[1 1 1] Destroys after Collision
  (if (Actor|ActorHasTag OtherActor "P1")
    (bind _asplayer_one (Utilities|Casting|CastToPlayerOne OtherActor))
    (if (not (Variables|/Game/BP/Characters/PlayerOne.PlayerOne_C|GetHasPickedUpSomething _asplayer_one))
      (Variables|/Game/BP/Characters/PlayerOne.PlayerOne_C|SetHomingMissilePickup _asplayer_one true)
      ;[1 1 1] DISENTEGRATION PS here
      (Effects|SpawnEmitteratLocation "/Game/Particles/Effects/PS_Pickup.PS_Pickup" (Transformation|GetWorldLocation (Variables|Default|GetSM_HomingJav)) :!label _label)
      (Audio|PlaySound2D "/Game/Sound/MSoundFiles/PickUps.PickUps" 1.0 1.0 0.0 0 0)
      (Actor|DestroyActor))
    (elif (Actor|ActorHasTag OtherActor "P2")
      (bind _asplayer_two (Utilities|Casting|CastToPlayerTwo OtherActor))
      (if (not (Variables|/Game/BP/Characters/PlayerTwo.PlayerTwo_C|GethasPickedUpSomething _asplayer_two))
        (Variables|/Game/BP/Characters/PlayerTwo.PlayerTwo_C|SetHomingMissilePickup _asplayer_two true)
        (goto _label)))))

(event Collision|EventActorBeginOverlap
  (params (OtherActor :type Actor%20Object%20Reference)))

(event EventTick
  (params (DeltaSeconds :type Float%20%28single-precision%29))
  (bind _startingrotation (Variables|Default|GetStartingRotation))
  ;[1 1 1] Just powerup Rotation and Translation
  (Transformation|AddLocalRotation (Variables|Default|GetSM_HomingJav) (Math|Rotator|MakeRotator (+ (.x _startingrotation) 1.5) (+ (.y _startingrotation) 2.0) (+ (.z _startingrotation) 0.5)) false false))

(event EventBeginPlay
  (bind _returnvalue (Transformation|GetActorTransform))
  ;[1 1 1] Begin Play
  (Variables|Default|SetStarting%20Pos (.location _returnvalue))
  (Variables|Default|SetStartingRotation (Math|Rotator|GetRotationXVector (.rotation _returnvalue)))
  ;[1 1 1] PS
  (Effects|SpawnEmitterAttached "/Game/PowerUps/RocketJav/Particles/PS_Javlin.PS_Javlin" (Variables|Default|GetForward%20Arrow) "None"))

(fn ConstructionScript)